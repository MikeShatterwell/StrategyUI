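; BP_AlphabetDataProvider is a test data provider that supplies one display item per character of an Alphabet string.
; GetDataItems constructs a BP_AlphabetDataItem for each character, sets its text and a color with randomized hue, and returns the accumulated AlphabetData array.
; The array is never cleared, so repeated calls append more items, and IsProviderReady always reports true.
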(fn GetDataItems
  (for _array_element (Utilities|String|GetCharacterArrayfromString (Variables|Default|GetAlphabet))
    (bind _returnvalue (Game|ConstructObjectfromClass "/StrategyUI/Test/Alphabet/BP_AlphabetDataItem.BP_AlphabetDataItem_C"))
    (Variables|/StrategyUI/Test/Alphabet/BP_AlphabetDataItem.BP_AlphabetDataItem_C|SetDisplayText _returnvalue (Utilities|Text|ToText(String) _array_element))
    (bind _output_get (Variables|/StrategyUI/Test/Alphabet/BP_AlphabetDataItem.BP_AlphabetDataItem_C|SetDisplayColor _returnvalue "(R=1.000000,G=0.222222,B=0.222222,A=1.000000)"))
    (Class|KismetMathLibrary|LinearColorSetRandomHue _output_get)
    (Utilities|Array|Add (LocalVariables|GetAlphabetData) _returnvalue))
  (return (LocalVariables|GetAlphabetData)))

(fn IsProviderReady
  (return true))