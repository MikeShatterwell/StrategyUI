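; Test data provider that supplies one display item per letter of an alphabet string.
; GetDataItems splits the string into characters and builds a BP_AlphabetDataItem for each, with the letter as display text and a randomized-hue color.
; Items are appended to AlphabetData on each call without clearing it first.
; Initialization creates the update delegate wrapper, whose validity also serves as the provider's readiness check.
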(event EventInitializeDataProvider
  (bind _returnvalue (Game|ConstructObjectfromClass "/Script/StrategyUI.OnDataProviderUpdatedDelegateWrapper"))
  (Variables|StrategyUI|Examples|SetDelegateWrapper _returnvalue))

(fn GetDataItems
  (for _array_element (Utilities|String|GetCharacterArrayfromString (Variables|StrategyUI|Examples|GetAlphabet))
    (bind _returnvalue (Game|ConstructObjectfromClass "/StrategyUI/Test/Data/Alphabet/BP_AlphabetDataItem.BP_AlphabetDataItem_C"))
    (Variables|/StrategyUI/Test/Data/Alphabet/BP_AlphabetDataItem.BP_AlphabetDataItem_C|SetDisplayText _returnvalue (Utilities|Text|ToText(String) _array_element))
    (bind _output_get (Variables|/StrategyUI/Test/Data/Alphabet/BP_AlphabetDataItem.BP_AlphabetDataItem_C|SetDisplayColor _returnvalue "(R=1.000000,G=0.222222,B=0.222222,A=1.000000)"))
    (Class|KismetMathLibrary|LinearColorSetRandomHue _output_get)
    (Utilities|Array|Add (LocalVariables|GetAlphabetData) _returnvalue))
  (return (LocalVariables|GetAlphabetData)))

(fn GetonDataProviderUpdated
  (return (Variables|StrategyUI|Examples|GetDelegateWrapper)))

(fn IsProviderReady
  (return (Utilities|IsValid (Variables|StrategyUI|Examples|GetDelegateWrapper))))